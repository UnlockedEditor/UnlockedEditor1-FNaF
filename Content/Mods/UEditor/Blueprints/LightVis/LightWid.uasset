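; LightWid is an actor in the UEditor mod that toggles widget markers for the Light actors in the level.
; ShowLights spawns an Attach actor at each Light's transform, hands that light to it and its widget as a reference, then attaches it to the light keeping world transforms.
; HideLights destroys every Attach actor in the level.
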(event Custom|Show%20Lights
  (bind _outactors (Actor|GetAllActorsOfClass "/Script/Engine.Light"))
  (for _array_element _outactors
    (bind _returnvalue (Game|SpawnActorfromClass "/Game/Mods/UEditor/Blueprints/LightVis/Attach.Attach_C" (Transformation|GetActorTransform _array_element) "Undefined" 0 0))
    (Variables|/Game/Mods/UEditor/Blueprints/LightVis/Attach.Attach_C|SetAttachedTo _returnvalue _array_element)
    (bind _aswidget (Utilities|Casting|CastToWidget (UserInterface|GetWidget (Variables|/Game/Mods/UEditor/Blueprints/LightVis/Attach.Attach_C|GetWidget _returnvalue))))
    (Variables|/Game/Mods/UEditor/Blueprints/LightVis/Widget.Widget_C|SetActorRef _aswidget _array_element)
    (Transformation|AttachActorToActor _returnvalue _array_element "None" "KeepWorld" "KeepWorld" "KeepWorld" true)))

(event Custom|HideLights
  (bind _outactors (Actor|GetAllActorsOfClass "/Game/Mods/UEditor/Blueprints/LightVis/Attach.Attach_C"))
  (for _array_element _outactors
    (Actor|DestroyActor _array_element)))

(event Collision|EventActorBeginOverlap
  (params (OtherActor :type Actor%20Object%20Reference)))

(event EventTick
  (params (DeltaSeconds :type Float%20%28single-precision%29)))

(fn ConstructionScript)