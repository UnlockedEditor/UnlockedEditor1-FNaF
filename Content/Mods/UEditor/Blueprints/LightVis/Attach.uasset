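; Attach is an editor-mod actor in the LightVis folder that shows a widget component tied to another object, likely as a light marker.
; Each Tick it hides the widget when the player pawn is beyond a fixed distance and shows it otherwise.
; It also destroys itself once its AttachedTo reference is no longer valid, so it does not outlive that object.
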(event EventBeginPlay)

(event Collision|EventActorBeginOverlap
  (params (OtherActor :type Actor%20Object%20Reference)))

(event EventTick
  (params (DeltaSeconds :type Float%20%28single-precision%29))
  (bind _widget (Variables|Default|GetWidget))
  (Utilities|FlowControl|Sequence
    (:then_0
      (if (> (Math|Vector|Distance(Vector) (Transformation|GetActorLocation) (Transformation|GetActorLocation (Game|Player|GetPlayerPawn 0))) 3.5e+03)
        (Rendering|SetVisibility _widget false false)
        (else
          (Rendering|SetVisibility _widget true false))))
    (:then_1
      (Utilities|IsValid (Variables|Default|GetAttachedTo)
        (:Is%20Not%20Valid
          (Actor|DestroyActor))))))

(fn ConstructionScript)